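; Turret actor that tracks player 0 and fires debug-drawn hitscan shots, only printing a message on a hit.
; Each Tick, hand-written horizontal distance and dot-product checks test range and a view cone around the current yaw.
; Inside the cone, TurretTop turns by wrapped-delta Lerp while a fire timer accumulates.
; Once the timer is ready and aim is within threshold, it line-traces from the computed muzzle toward the player.
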(event `self.ReceiveBeginPlay`
  (bind (_returnvalue_roll _returnvalue_pitch _returnvalue_yaw) (`KismetMathLibrary.BreakRotator` (`SceneComponent.K2_GetComponentRotation` (`self.TurretTop`))))
  (set `self.YawActual` _returnvalue_yaw))

(event `self.ReceiveTick`
  (params (DeltaSeconds :type "Float (single-precision)"))
  (bind _returnvalue (`self.K2_GetActorLocation` (`GameplayStatics.GetPlayerPawn` 0)))
  (bind (_returnvalue_x _returnvalue_y) (`KismetMathLibrary.BreakVector` (- _returnvalue (`SceneComponent.K2_GetComponentLocation` (`self.TurretTop`)))))
  (bind _returnvalue_2 (+ (`SceneComponent.K2_GetComponentLocation` (`self.TurretTop`)) (* (`KismetMathLibrary.MakeVector` (`KismetMathLibrary.DegCos` (`self.YawActual`)) (`KismetMathLibrary.DegSin` (`self.YawActual`))) (`self.LongitudCanon`)) (`KismetMathLibrary.MakeVector` 0.0 0.0 (`self.AlturaCanon`))))
  (bind _returnvalue_3 (- _returnvalue _returnvalue_2))
  (bind _x (.x _returnvalue_3))
  (bind _y (.y _returnvalue_3))
  (bind _z (.z _returnvalue_3))
  (bind _output_get (set `self.Distancia` (`KismetMathLibrary.Sqrt` (+ (* _returnvalue_x _returnvalue_x) (* _returnvalue_y _returnvalue_y)))))
  (if (<= _output_get (`self.RangoVision`))
    (bind _output_get_2 (set `self.DirX` (/ _returnvalue_x _output_get)))
    (bind _output_get_3 (set `self.DirY` (/ _returnvalue_y _output_get)))
    (if (<= (`KismetMathLibrary.DegAcos` (+ (* (`KismetMathLibrary.DegCos` (`self.YawActual`)) _output_get_2) (* (`KismetMathLibrary.DegSin` (`self.YawActual`)) _output_get_3))) (`self.AnguloCono`))
      (bind _output_get_4 (set `self.Delta` (- (`KismetMathLibrary.DegAtan2` (`self.DirY`) (`self.DirX`)) (`self.YawActual`))))
      (if (> _output_get_4 180.0)
        (set `self.Delta` (- (`self.Delta`) 360.0)))
      (if (< (`self.Delta`) -180.0)
        (set `self.Delta` (+ (`self.Delta`) 360.0)))
      (bind _output_get_5 (set `self.YawActual` (`KismetMathLibrary.Lerp` (`self.YawActual`) (+ (`self.YawActual`) (`self.Delta`)) (`KismetMathLibrary.FClamp` (* DeltaSeconds (`self.VelocidadGiro`))))))
      (`SceneComponent.K2_SetWorldRotation` (`self.TurretTop`) (`KismetMathLibrary.MakeRotator` 0.0 0.0 _output_get_5) false false)
      (set `self.TiempoDisparo` (+ (`self.TiempoDisparo`) DeltaSeconds))
      (if (and (>= (`self.TiempoDisparo`) (`self.Cadencia`)) (<= (`KismetMathLibrary.Abs` (`self.Delta`)) (`self.UmbralDisparo`)))
        (bind _outhit (`KismetSystemLibrary.LineTraceSingle` :`Start` _returnvalue_2 :`End` (+ _returnvalue_2 (* (/ _returnvalue_3 (`KismetMathLibrary.Sqrt` (+ (* _x _x) (* _y _y) (* _z _z)))) (`self.RangoVision`))) :`TraceChannel` "TraceTypeQuery1" :`DrawDebugType` "ForDuration"))
        (set `self.TiempoDisparo` 0.0)
        (if (== (`.HitActor` (`GameplayStatics.BreakHitResult` _outhit)) (`GameplayStatics.GetPlayerPawn` 0))
          (`KismetSystemLibrary.PrintString` "Le ha dado"))))))

(fn `UserConstructionScript`)